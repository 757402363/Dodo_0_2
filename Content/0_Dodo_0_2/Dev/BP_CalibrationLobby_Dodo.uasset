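; BP_CalibrationLobby_Dodo is the lobby that calibrates the player's right-hand finger-tracking range before opening the next map.
; Overlapping the true sphere records per-step min/max finger values on the PlayerController and advances; the false sphere steps back.
; Each step drives the guide widget and hand AnimBP, with a PlayAsPC debug path skipping the VR right-controller cast.
; Touching the magic circle after calibration triggers an easter egg changing music, materials and collision.
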(event `self.ReceiveBeginPlay`
  ;[1 1 1] 开始运行时，获得相关引用，并开始显示引导内容
  (`|ExecutionSequence`
    (:`then_0`
      ;;[0 0 0] 玩家控制器
      (bind _asplayer_controller_dodo (cast `/Game/0_Dodo_0_2/Core/PlayerController_Dodo` (`GameplayStatics.GetPlayerController` 0)))
      (set `self.PlayerController_Dodo` _asplayer_controller_dodo))
    (:`then_1`
      ;;[0 0 0] 游戏实例
      (bind _asgame_instance_dodo (cast `/Game/0_Dodo_0_2/Core/GameInstance_Dodo` (`GameplayStatics.GetGameInstance`)))
      (set `self.GameInstance_Dodo` _asgame_instance_dodo))
    (:`then_2`
      ;;[0 0 0] 校准引导UI
      (bind _asumg_calibration_guide_dodo (cast `/Game/0_Dodo_0_2/UI/UMG/UMG_CalibrationGuide_Dodo` (`WidgetComponent.GetUserWidgetObject` (`self.WidgetComp_CalibrationGuide`))))
      (set `self.UMG_CalibrationGuide_Dodo` _asumg_calibration_guide_dodo))
    (:`then_3`
      ;;[0 0 0] 校准引导骨骼动画
      (bind _asanim_bp_guide_hand_dodo (cast `/Game/0_Dodo_0_2/Characters/VRPawn/VirtualReality/Mannequin/Animations/AnimBP_GuideHand_Dodo` (`SkeletalMeshComponent.GetAnimInstance` (`self.GuideHand`))))
      (set `self.AnimBP_GuideHand_Dodo` _asanim_bp_guide_hand_dodo))
    (:`then_4`
      ;;[0 0 0] 引导内容
      (`self.GuideContents`)
      ;;[0 0 0] 延迟0.5s开始播放背景音乐
      (`KismetSystemLibrary.Delay` 0.5)
      (`AudioComponent.Play` (`self.Sound_BGM`) 0.0)
      (`AudioComponent.AdjustVolume` (`self.Sound_BGM`) 0.0 (`self.BGM_DefaultSoundVolume`) "Linear"))))

(event `self.ReceiveTick`
  (params (DeltaSeconds :type "Float (single-precision)"))
  ;[1 1 1] 两个校准交互球体旋转
  (`SceneComponent.K2_AddWorldRotation` (`self.SM_Calibration_True`) (struct :`Pitch` 0.2 :`Yaw` -0.2 :`Roll` -0.2) false false)
  (`SceneComponent.K2_AddWorldRotation` (`self.SM_Calibration_False`) (struct :`Pitch` -0.2 :`Yaw` 0.2 :`Roll` 0.2) false false))

(event `SM_Calibration_Feedback`
  (params (SM_Calibration :type "StaticMeshComponent Object Reference"))
  ;[1 1 1] 校准交互球体的反馈
  (bind (_direction _line0) (`Timeline|OverlapFeedback` :!via `PlayFromStart`)
    (:`Update`
      (bind _returnvalue (`KismetMathLibrary.MapRangeClamped` _line0 0.0 1.0 0.35 0.38))
      (`SceneComponent.SetRelativeScale3D` SM_Calibration (`KismetMathLibrary.MakeVector` _returnvalue _returnvalue _returnvalue)))))

(event `GuideContents`
  (bind _calibrationstep (`self.CalibrationStep`))
  ;[1 1 1] 根据校准步骤设置引导内容
  (`/Game/0_Dodo_0_2/UI/UMG/UMG_CalibrationGuide_Dodo.GuideText` (`self.UMG_CalibrationGuide_Dodo`) _calibrationstep)
  (set `/Game/0_Dodo_0_2/Characters/VRPawn/VirtualReality/Mannequin/Animations/AnimBP_GuideHand_Dodo.CalibrationStep` (`KismetMathLibrary.Conv_IntToDouble` _calibrationstep) (`self.AnimBP_GuideHand_Dodo`)))

(event `self.Collision_True.OnComponentBeginOverlap`
  (params (OverlappedComponent :type "PrimitiveComponent Object Reference") (OtherActor :type "Actor Object Reference") (OtherComp :type "PrimitiveComponent Object Reference") (OtherBodyIndex :type Integer) (bFromSweep :type Boolean) (SweepResult :type "HitResult Structure (by ref)"))
  (bind _playercontroller_dodo (`self.PlayerController_Dodo`))
  (bind _playercontroller_dodo_2 (`self.PlayerController_Dodo`))
  (bind _playercontroller_dodo_3 (`self.PlayerController_Dodo`))
  (bind _playercontroller_dodo_4 (`self.PlayerController_Dodo`))
  (bind _playercontroller_dodo_5 (`self.PlayerController_Dodo`))
  (bind _calibrationstep (`self.CalibrationStep`))
  (bind _playercontroller_dodo_6 (`self.PlayerController_Dodo`))
  (bind _data_righthand (`/Game/0_Dodo_0_2/Core/PlayerController_Dodo.Data_RightHand` _playercontroller_dodo))
  (bind _data_righthand_2 (`/Game/0_Dodo_0_2/Core/PlayerController_Dodo.Data_RightHand` _playercontroller_dodo_3))
  (bind _data_righthand_3 (`/Game/0_Dodo_0_2/Core/PlayerController_Dodo.Data_RightHand` _playercontroller_dodo_4))
  (bind _data_righthand_4 (`/Game/0_Dodo_0_2/Core/PlayerController_Dodo.Data_RightHand` _playercontroller_dodo_6))
  ;[1 1 1] （蓝色球体）校准数据捕捉，并设置引导内容等
  ;;[0 0 0] 判断是作为PCPawn（调试）还是作为VRPawn
  (if (not (`.PlayAsPC_46_082C2DDF49E63916865F99A1A9B5F771` (break `/Game/0_Dodo_0_2/Dev/Structure/Struc_VRPlayerSettings` (`/Game/0_Dodo_0_2/Core/GameInstance_Dodo.Struc_VRPlayerSettings` (`self.GameInstance_Dodo`)))))
    ;;[0 0 0] 获得对右手的引用
    (bind _asbp_motion_controller_right (cast `/Game/0_Dodo_0_2/Characters/VRPawn/BP_MotionController_Right` OtherActor))
    (`/Engine/EditorBlueprintResources/StandardMacros.IsValid` (`self.BP_MotionController_Right`)
      (:`Is Valid`
        _)
      (:`Is Not Valid`
        (set `self.BP_MotionController_Right` _asbp_motion_controller_right))))
  (`|ExecutionSequence`
    (:`then_0`
      (switch `int` (`self.CalibrationStep`)
        (:`1`
          ;;[0 0 0] 数据捕捉1
          (set `/Game/0_Dodo_0_2/Core/PlayerController_Dodo.Data_Max_Thumb_Yaw` (`KismetMathLibrary.Conv_IntToDouble` (`|GetArrayItem` _data_righthand)) _playercontroller_dodo)
          (set `/Game/0_Dodo_0_2/Core/PlayerController_Dodo.Data_Max_Index_Yaw` (`KismetMathLibrary.Conv_IntToDouble` (`|GetArrayItem` _data_righthand 3)) _playercontroller_dodo)
          (set `/Game/0_Dodo_0_2/Core/PlayerController_Dodo.Data_Max_Index_Pitch1` (`KismetMathLibrary.Conv_IntToDouble` (`|GetArrayItem` _data_righthand 4)) _playercontroller_dodo)
          (set `/Game/0_Dodo_0_2/Core/PlayerController_Dodo.Data_Max_Index_Pitch2` (`KismetMathLibrary.Conv_IntToDouble` (`|GetArrayItem` _data_righthand 5)) _playercontroller_dodo)
          (set `/Game/0_Dodo_0_2/Core/PlayerController_Dodo.Data_Max_Middle_Pitch1` (`KismetMathLibrary.Conv_IntToDouble` (`|GetArrayItem` _data_righthand 7)) _playercontroller_dodo)
          (set `/Game/0_Dodo_0_2/Core/PlayerController_Dodo.Data_Max_Middle_Pitch2` (`KismetMathLibrary.Conv_IntToDouble` (`|GetArrayItem` _data_righthand 8)) _playercontroller_dodo)
          (set `/Game/0_Dodo_0_2/Core/PlayerController_Dodo.Data_Min_Ring_Yaw` (`KismetMathLibrary.Conv_IntToDouble` (`|GetArrayItem` _data_righthand 9)) _playercontroller_dodo)
          (set `/Game/0_Dodo_0_2/Core/PlayerController_Dodo.Data_Max_Ring_Pitch1` (`KismetMathLibrary.Conv_IntToDouble` (`|GetArrayItem` _data_righthand 10)) _playercontroller_dodo)
          (set `/Game/0_Dodo_0_2/Core/PlayerController_Dodo.Data_Max_Ring_Pitch2` (`KismetMathLibrary.Conv_IntToDouble` (`|GetArrayItem` _data_righthand 11)) _playercontroller_dodo)
          (set `/Game/0_Dodo_0_2/Core/PlayerController_Dodo.Data_Min_Pinky_Yaw` (`KismetMathLibrary.Conv_IntToDouble` (`|GetArrayItem` _data_righthand 12)) _playercontroller_dodo)
          (set `/Game/0_Dodo_0_2/Core/PlayerController_Dodo.Data_Max_Pinky_Pitch1` (`KismetMathLibrary.Conv_IntToDouble` (`|GetArrayItem` _data_righthand 13)) _playercontroller_dodo)
          (set `/Game/0_Dodo_0_2/Core/PlayerController_Dodo.Data_Max_Pinky_Pitch2` (`KismetMathLibrary.Conv_IntToDouble` (`|GetArrayItem` _data_righthand 14)) _playercontroller_dodo))
        (:`2`
          ;;[0 0 0] 数据捕捉2
          (set `/Game/0_Dodo_0_2/Core/PlayerController_Dodo.Data_Min_Thumb_Yaw` (`KismetMathLibrary.Conv_IntToDouble` (`|GetArrayItem` _data_righthand_2)) _playercontroller_dodo_3)
          (set `/Game/0_Dodo_0_2/Core/PlayerController_Dodo.Data_Max_Thumb_Pitch1` (`KismetMathLibrary.Conv_IntToDouble` (`|GetArrayItem` _data_righthand_2 1)) _playercontroller_dodo_3)
          (set `/Game/0_Dodo_0_2/Core/PlayerController_Dodo.Data_Max_Thumb_Pitch2` (`KismetMathLibrary.Conv_IntToDouble` (`|GetArrayItem` _data_righthand_2 2)) _playercontroller_dodo_3)
          (set `/Game/0_Dodo_0_2/Core/PlayerController_Dodo.Data_Min_Index_Yaw` (`KismetMathLibrary.Conv_IntToDouble` (`|GetArrayItem` _data_righthand_2 3)) _playercontroller_dodo_3)
          (set `/Game/0_Dodo_0_2/Core/PlayerController_Dodo.Data_Max_Ring_Yaw` (`KismetMathLibrary.Conv_IntToDouble` (`|GetArrayItem` _data_righthand_2 9)) _playercontroller_dodo_3)
          (set `/Game/0_Dodo_0_2/Core/PlayerController_Dodo.Data_Max_Pinky_Yaw` (`KismetMathLibrary.Conv_IntToDouble` (`|GetArrayItem` _data_righthand_2 12)) _playercontroller_dodo_3))
        (:`3`
          ;;[0 0 0] 数据捕捉3
          (set `/Game/0_Dodo_0_2/Core/PlayerController_Dodo.Data_Min_Index_Pitch1` (`KismetMathLibrary.Conv_IntToDouble` (`|GetArrayItem` _data_righthand_4 4)) _playercontroller_dodo_6)
          (set `/Game/0_Dodo_0_2/Core/PlayerController_Dodo.Data_Min_Index_Pitch2` (`KismetMathLibrary.Conv_IntToDouble` (`|GetArrayItem` _data_righthand_4 5)) _playercontroller_dodo_6)
          (set `/Game/0_Dodo_0_2/Core/PlayerController_Dodo.Data_Min_Middle_Pitch1` (`KismetMathLibrary.Conv_IntToDouble` (`|GetArrayItem` _data_righthand_4 7)) _playercontroller_dodo_6)
          (set `/Game/0_Dodo_0_2/Core/PlayerController_Dodo.Data_Min_Middle_Pitch2` (`KismetMathLibrary.Conv_IntToDouble` (`|GetArrayItem` _data_righthand_4 8)) _playercontroller_dodo_6)
          (set `/Game/0_Dodo_0_2/Core/PlayerController_Dodo.Data_Min_Ring_Pitch1` (`KismetMathLibrary.Conv_IntToDouble` (`|GetArrayItem` _data_righthand_4 10)) _playercontroller_dodo_6)
          (set `/Game/0_Dodo_0_2/Core/PlayerController_Dodo.Data_Min_Ring_Pitch2` (`KismetMathLibrary.Conv_IntToDouble` (`|GetArrayItem` _data_righthand_4 11)) _playercontroller_dodo_6)
          (set `/Game/0_Dodo_0_2/Core/PlayerController_Dodo.Data_Min_Pinky_Pitch1` (`KismetMathLibrary.Conv_IntToDouble` (`|GetArrayItem` _data_righthand_4 13)) _playercontroller_dodo_6)
          (set `/Game/0_Dodo_0_2/Core/PlayerController_Dodo.Data_Min_Pinky_Pitch2` (`KismetMathLibrary.Conv_IntToDouble` (`|GetArrayItem` _data_righthand_4 14)) _playercontroller_dodo_6))
        (:`4`
          ;;[0 0 0] 数据捕捉4
          (set `/Game/0_Dodo_0_2/Core/PlayerController_Dodo.Data_Min_Thumb_Pitch1` (`KismetMathLibrary.Conv_IntToDouble` (`|GetArrayItem` _data_righthand_3 1)) _playercontroller_dodo_4)
          (set `/Game/0_Dodo_0_2/Core/PlayerController_Dodo.Data_Min_Thumb_Pitch2` (`KismetMathLibrary.Conv_IntToDouble` (`|GetArrayItem` _data_righthand_3 2)) _playercontroller_dodo_4))
        (:`5`
          ;;[0 0 0] 数据捕捉5
          (set `/Game/0_Dodo_0_2/Core/PlayerController_Dodo.Data_Min_Middle_Yaw` (`KismetMathLibrary.Conv_IntToDouble` (`|GetArrayItem` (`/Game/0_Dodo_0_2/Core/PlayerController_Dodo.Data_RightHand` _playercontroller_dodo_5) 6)) _playercontroller_dodo_5))
        (:`6`
          ;;[0 0 0] 数据捕捉6
          (set `/Game/0_Dodo_0_2/Core/PlayerController_Dodo.Data_Max_Middle_Yaw` (`KismetMathLibrary.Conv_IntToDouble` (`|GetArrayItem` (`/Game/0_Dodo_0_2/Core/PlayerController_Dodo.Data_RightHand` _playercontroller_dodo_2) 6)) _playercontroller_dodo_2)
          ;;[0 0 0] 校准完成
          (set `/Game/0_Dodo_0_2/Core/PlayerController_Dodo.CalibrationOK` true _playercontroller_dodo_2)
          ;;[0 0 0] 彩蛋，校准完毕后出现一个极小的魔法阵特效
          (`SceneComponent.SetVisibility` (`self.ActorComp_MagicCircle`) true false))
        (:`7`
          ;;[0 0 0] 确认校准效果后退出校准关卡（摄像机淡化，背景音乐调整音量）
          (`PlayerCameraManager.StartCameraFade` (`GameplayStatics.GetPlayerCameraManager` 0) 0.0 1.0 1.5 (struct :`R` 1.0 :`G` 1.0 :`B` 1.0 :`A` 1.0) false true)
          (`AudioComponent.AdjustVolume` (`self.Sound_BGM`) 1.5 0.0 "Linear")
          (`KismetSystemLibrary.Delay` 1.5)
          (`GameplayStatics.OpenLevelBySoftObjectPtr` "/Game/0_Dodo_0_2/Maps/Map_Temp.Map_Temp"))))
    (:`then_1`
      ;;[0 0 0] 校准交互球体反馈
      (`self.SM_Calibration_Feedback` (`self.SM_Calibration_True`))
      ;;[0 0 0] 进入下一校准步骤并显示引导内容
      (if (< _calibrationstep 7)
        (set `self.CalibrationStep` (+ _calibrationstep 1))
        (`self.GuideContents`)))))

(event `self.Collision_False.OnComponentBeginOverlap`
  (params (OverlappedComponent :type "PrimitiveComponent Object Reference") (OtherActor :type "Actor Object Reference") (OtherComp :type "PrimitiveComponent Object Reference") (OtherBodyIndex :type Integer) (bFromSweep :type Boolean) (SweepResult :type "HitResult Structure (by ref)"))
  (bind _calibrationstep (`self.CalibrationStep`))
  ;[1 1 1] （红色球体）返回上一校准步骤，并设置引导内容等
  ;;[0 0 0] 判断是作为PCPawn（调试）还是作为VRPawn
  (if (not (`.PlayAsPC_46_082C2DDF49E63916865F99A1A9B5F771` (break `/Game/0_Dodo_0_2/Dev/Structure/Struc_VRPlayerSettings` (`/Game/0_Dodo_0_2/Core/GameInstance_Dodo.Struc_VRPlayerSettings` (`self.GameInstance_Dodo`)))))
    ;;[0 0 0] 获得对右手的引用
    (bind _asbp_motion_controller_right (cast `/Game/0_Dodo_0_2/Characters/VRPawn/BP_MotionController_Right` OtherActor))
    (`/Engine/EditorBlueprintResources/StandardMacros.IsValid` (`self.BP_MotionController_Right`)
      (:`Is Valid`
        _)
      (:`Is Not Valid`
        (set `self.BP_MotionController_Right` _asbp_motion_controller_right))))
  ;;[0 0 0] 校准交互球体反馈
  (`self.SM_Calibration_Feedback` (`self.SM_Calibration_False`))
  (`|ExecutionSequence`
    (:`then_0`
      ;;[0 0 0] 如果当前为第7步（即观察校准效果），返回上一步前需要将CalibrationOK设置为False
      (if (== _calibrationstep 7)
        (set `/Game/0_Dodo_0_2/Core/PlayerController_Dodo.CalibrationOK` false (`self.PlayerController_Dodo`))
        ;;[0 0 0] 彩蛋相关，取消校准完毕状态后特效不可视
        (`SceneComponent.SetVisibility` (`self.ActorComp_MagicCircle`) false false)))
    (:`then_1`
      ;;[0 0 0] 返回上一校准步骤并显示引导内容
      (if (> _calibrationstep 0)
        (set `self.CalibrationStep` (- _calibrationstep 1))
        (`self.GuideContents`)))))

(event `self.Collision_MagicCircle.OnComponentBeginOverlap`
  (params (OverlappedComponent :type "PrimitiveComponent Object Reference") (OtherActor :type "Actor Object Reference") (OtherComp :type "PrimitiveComponent Object Reference") (OtherBodyIndex :type Integer) (bFromSweep :type Boolean) (SweepResult :type "HitResult Structure (by ref)"))
  (bind _sm_lobby (`self.SM_Lobby`))
  (bind _sm_calibration_false (`self.SM_Calibration_False`))
  (bind _egg_material (`self.Egg_Material`))
  (bind _sm_calibration_true (`self.SM_Calibration_True`))
  (bind _guidehand (`self.GuideHand`))
  (bind _bp_motioncontroller_right (`self.BP_MotionController_Right`))
  ;[1 1 1] 彩蛋
  ;;[0 0 0] 判断是作为PCPawn（调试）还是作为VRPawn
  (if (not (`.PlayAsPC_46_082C2DDF49E63916865F99A1A9B5F771` (break `/Game/0_Dodo_0_2/Dev/Structure/Struc_VRPlayerSettings` (`/Game/0_Dodo_0_2/Core/GameInstance_Dodo.Struc_VRPlayerSettings` (`self.GameInstance_Dodo`)))))
    (cast `/Game/0_Dodo_0_2/Characters/VRPawn/BP_MotionController_Right` OtherActor))
  ;;[0 0 0] 如果与此碰撞体重叠时校准已完毕，销毁碰撞体避免再产生相关交互
  (if (`/Game/0_Dodo_0_2/Core/PlayerController_Dodo.CalibrationOK` (`self.PlayerController_Dodo`))
    (`ActorComponent.K2_DestroyComponent` (`self.Collision_MagicCircle`))
    (`ActorComponent.K2_DestroyComponent` (`self.Collision_True`))
    (`ActorComponent.K2_DestroyComponent` (`self.Collision_False`))
    ;;[0 0 0] 放大魔法阵特效并更换背景音乐，预留一点时间观看
    (`AudioComponent.AdjustVolume` (`self.Sound_BGM`) 1.5 0.0 "Linear")
    (`KismetSystemLibrary.Delay` 1.5)
    (set `AudioComponent.Sound` "/Game/0_Dodo_0_2/Sounds/Sound_AT_KulveTaroth_3.Sound_AT_KulveTaroth_3" (`self.Sound_BGM`))
    (`AudioComponent.Play` (`self.Sound_BGM`) 0.0)
    (`AudioComponent.AdjustVolume` (`self.Sound_BGM`) 1.5 (`self.BGM_DefaultSoundVolume`) "Linear")
    (bind (_direction _line0) (`Timeline|MagicCircleChange` :!via `PlayFromStart`)
      (:`Update`
        (`SceneComponent.SetWorldScale3D` (`self.ActorComp_MagicCircle`) (`KismetMathLibrary.MakeVector` _line0 _line0 _line0)))
      (:`Finished`
        (`KismetSystemLibrary.Delay` 5.0)
        ;;[0 0 0] 摄像机画面渐白，然后对组件进行设置（销毁，或改变材质、碰撞属性），再将摄像机画面和背景音乐渐渐恢复。（注意此处不能用“序列”将操作分开，经测试“序列”引脚编号靠后的节点不会等待编号靠前的“延迟”结束就会执行）
        (`PlayerCameraManager.StartCameraFade` (`GameplayStatics.GetPlayerCameraManager` 0) 0.0 1.0 1.5 (struct :`R` 1.0 :`G` 1.0 :`B` 1.0 :`A` 1.0) false true)
        (`KismetSystemLibrary.Delay` 1.5)
        (`ActorComponent.K2_DestroyComponent` (`self.PointLight`))
        (`ActorComponent.K2_DestroyComponent` (`self.SpotLight`))
        (`ActorComponent.K2_DestroyComponent` (`self.WidgetComp_CalibrationGuide`))
        (`ActorComponent.K2_DestroyComponent` (`self.ActorComp_MagicCircle`))
        (for _index (range (`PrimitiveComponent.GetNumMaterials` _sm_lobby))
          (`PrimitiveComponent.SetMaterial` _sm_lobby _index _egg_material)
          (`PrimitiveComponent.SetMaterial` _sm_calibration_true 0 _egg_material)
          (`PrimitiveComponent.SetMaterial` _sm_calibration_false 0 _egg_material)
          (`PrimitiveComponent.SetMaterial` _guidehand 0 _egg_material)
          (`/Engine/EditorBlueprintResources/StandardMacros.IsValid` _bp_motioncontroller_right
            (:`Is Valid`
              (`PrimitiveComponent.SetMaterial` (`/Game/0_Dodo_0_2/Characters/VRPawn/BP_MotionController_Right.HandMesh` _bp_motioncontroller_right) 0 _egg_material))
            (:`Is Not Valid`
              _))
          (`PrimitiveComponent.SetCollisionEnabled` _sm_lobby "NoCollision")
          (`PrimitiveComponent.SetCollisionEnabled` _sm_calibration_true "NoCollision")
          (`PrimitiveComponent.SetCollisionEnabled` _sm_calibration_false "NoCollision")
          (`PrimitiveComponent.SetCollisionEnabled` _guidehand "NoCollision")
          (`KismetSystemLibrary.Delay` 0.5)
          (`PlayerCameraManager.StartCameraFade` (`GameplayStatics.GetPlayerCameraManager` 0) 1.0 0.0 1.5 (struct :`R` 1.0 :`G` 1.0 :`B` 1.0 :`A` 1.0) false false)
          (`AudioComponent.AdjustVolume` (`self.Sound_BGM`) 1.5 0.0 "Linear")
          (`KismetSystemLibrary.Delay` 1.5)
          (set `AudioComponent.Sound` "/Game/0_Dodo_0_2/Sounds/Sound_SuccessionOfLight.Sound_SuccessionOfLight" (`self.Sound_BGM`))
          (`AudioComponent.Play` (`self.Sound_BGM`) 27.0)
          (`AudioComponent.AdjustVolume` (`self.Sound_BGM`) 1.5 (`self.BGM_DefaultSoundVolume`) "Linear"))))))

(event `self.Sound_BGM.OnAudioFinished`
  ;[1 1 1] 背景音乐循环
  (`AudioComponent.Play` (`self.Sound_BGM`) 0.0))

(fn `UserConstructionScript`)